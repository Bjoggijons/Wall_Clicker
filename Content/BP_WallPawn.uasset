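; BP_WallPawn is a pawn that enables mouse clicking, shows the upgrades UI and spawns successive walls.
; BeginPlay creates the UI_Upgrades widget and starts a looping one-second timer with no function name shown.
; SpawnWall waits a second, then spawns a BP_Wall with health and material from the current Walllist entry.
; It then advances WallCount and adds a fixed amount to the UI's HealthBar value.
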(event Custom|SpawnWall
  (params (SpawnTransform :type Transform))
  (bind _wall_list (Variables|Default|Getwall-list))
  (bind _ui_ref (Variables|Default|GetUI_Ref))
  (bind _wall_count (Variables|Default|Getwall%20count))
  (bind _output (Utilities|Array|Get(acopy) _wall_list _wall_count))
  (Utilities|FlowControl|Delay 1.0)
  (bind _returnvalue (Game|SpawnActorfromClass "/Game/BP_Wall.BP_Wall_C" SpawnTransform "Undefined" "MultiplyWithRoot" 0 (.wall-health _output) (Math|Conversions|ToFloat(Integer) (.wall-health _output)) 0))
  (Rendering|Material|SetMaterial (Variables|/Game/BP_Wall.BP_Wall_C|GetCube _returnvalue) 0 (.wall-mat _output))
  (Math|Integer|IncrementInt (Variables|Default|Getwall%20count)
    (:%20%20
      (Variables|/Game/UI_Upgrades.UI_Upgrades_C|SetHealth_Bar _ui_ref (+ (Variables|/Game/UI_Upgrades.UI_Upgrades_C|GetHealth_Bar _ui_ref) 100)))))

(event EventBeginPlay
  (Variables|/Script/Engine.PlayerController|SetbEnableClickEvents (Game|GetPlayerController 0) true)
  (Variables|/Script/Engine.PlayerController|SetbShowMouseCursor (Game|GetPlayerController 0) true)
  (Utilities|Time|SetTimerbyFunctionName 0 "" 1.0 true)
  (bind _returnvalue (UserInterface|CreateWidget "/Game/UI_Upgrades.UI_Upgrades_C"))
  (bind _output_get (Variables|Default|SetUI_Ref _returnvalue))
  (UserInterface|Viewport|AddtoViewport _output_get 0))

(fn ConstructionScript)