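; Clickable wall actor for a clicker game that loses health and earns the player money with each hit.
; On BeginPlay it caches BP_WallPawn after a short delay and registers itself with the pawn's UI.
; Clicks apply the pawn's Strength, update the health bar and, at zero health, spawn a replacement and destroy the wall.
; PerformClickAction applies auto-click damage and respawns likewise, but neither destroys the wall nor updates the bar.
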(event OnClicked(Cube)
  (params (TouchedComponent :type Primitive%20Component%20Object%20Reference) (ButtonPressed :type Key%20Structure :default "None"))
  (bind _wallpawn_ref (Variables|Default|GetWallPawn_Ref))
  (Audio|PlaySound2D "/Game/UI_SFX_Free_Pack/Wavs/Buttons/button_press_699.button_press_699" 1.0 1.0 0.0 0 0)
  (Variables|Default|SetWall_Health (- (Variables|Default|GetWall_Health) (Variables|/Game/BP_WallPawn.BP_WallPawn_C|GetStrength (Variables|Default|GetWallPawn_Ref))))
  (Variables|/Game/UI_Upgrades.UI_Upgrades_C|SetHealth_Bar (Variables|/Game/BP_WallPawn.BP_WallPawn_C|GetUI_Ref (Variables|Default|GetWallPawn_Ref)) (- (Variables|Default|GetWall_Health) (Variables|/Game/BP_WallPawn.BP_WallPawn_C|GetStrength (Variables|Default|GetWallPawn_Ref))))
  (Variables|/Game/BP_WallPawn.BP_WallPawn_C|SetMoney _wallpawn_ref (+ (Variables|/Game/BP_WallPawn.BP_WallPawn_C|GetMoney _wallpawn_ref) (Variables|/Game/BP_WallPawn.BP_WallPawn_C|GetStrength _wallpawn_ref)))
  (if (<= (Variables|Default|GetWall_Health) 0)
    (Default|SpawnWall (Variables|Default|GetWallPawn_Ref) (Transformation|GetActorTransform))
    (Actor|DestroyActor)
    (Variables|/Game/UI_Upgrades.UI_Upgrades_C|SetHealth_Bar (Variables|/Game/BP_WallPawn.BP_WallPawn_C|GetUI_Ref (Variables|Default|GetWallPawn_Ref)) 100)
    (Audio|PlaySound2D "/Game/StarterContent/Audio/Explosion02.Explosion02" 1.0 1.0 0.0 0 0)))

(event EventBeginPlay
  (Utilities|FlowControl|Delay 0.2)
  (bind _asbp_wall_pawn (Utilities|Casting|CastToBP_WallPawn (Game|Player|GetPlayerPawn 0)))
  (bind _output_get (Variables|Default|SetWallPawn_Ref _asbp_wall_pawn))
  (Variables|/Game/UI_Upgrades.UI_Upgrades_C|SetAs%20BP%20Wall (Variables|/Game/BP_WallPawn.BP_WallPawn_C|GetUI_Ref _output_get) self))

(fn ConstructionScript)

(fn PerformClickAction
  (bind _wallpawn_ref (Variables|Default|GetWallPawn_Ref))
  (Variables|Default|SetWall_Health (- (Variables|Default|GetWall_Health) (Variables|Default|GetAutoClickStrenght)))
  (Variables|/Game/BP_WallPawn.BP_WallPawn_C|SetMoney _wallpawn_ref (+ (Variables|/Game/BP_WallPawn.BP_WallPawn_C|GetMoney _wallpawn_ref) (Variables|Default|GetAutoClickStrenght)))
  (if (<= (Variables|Default|GetWall_Health) 0)
    (Default|SpawnWall (Variables|Default|GetWallPawn_Ref) (Transformation|GetActorTransform))))